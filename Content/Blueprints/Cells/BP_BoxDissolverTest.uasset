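; Test actor that drives a box-shaped dissolve volume through the PC_BoxDissolver_Data material parameter collection.
; It writes the DissolverShape component's world location, scale and forward, right and up vectors into the collection, describing an oriented box for materials that read it.
; The same writes run in the construction script and every Tick, updating the data both on construction and as the shape moves at runtime.
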(event EventTick
  (params (DeltaSeconds :type Float%20%28single-precision%29))
  (bind _dissolver__shape (Variables|Default|GetDissolver%20%20Shape))
  (bind _dissolver__shape_2 (Variables|Default|GetDissolver%20%20Shape))
  (Rendering|Material|SetVectorParameterValue "/Game/Art/Materials/BaseMaterials/PC_BoxDissolver_Data.PC_BoxDissolver_Data" "Location" (Math|Conversions|ToLinearColor(Vector) (Transformation|GetWorldLocation _dissolver__shape)) :!class /Script/Engine.KismetMaterialLibrary)
  (Rendering|Material|SetVectorParameterValue "/Game/Art/Materials/BaseMaterials/PC_BoxDissolver_Data.PC_BoxDissolver_Data" "Bounds" (Math|Conversions|ToLinearColor(Vector) (Transformation|GetWorldScale _dissolver__shape)) :!class /Script/Engine.KismetMaterialLibrary)
  (Rendering|Material|SetVectorParameterValue "/Game/Art/Materials/BaseMaterials/PC_BoxDissolver_Data.PC_BoxDissolver_Data" "Forward" (Math|Conversions|ToLinearColor(Vector) (Math|Vector|GetForwardVector _dissolver__shape_2)) :!class /Script/Engine.KismetMaterialLibrary)
  (Rendering|Material|SetVectorParameterValue "/Game/Art/Materials/BaseMaterials/PC_BoxDissolver_Data.PC_BoxDissolver_Data" "Right" (Math|Conversions|ToLinearColor(Vector) (Math|Vector|GetRightVector _dissolver__shape_2)) :!class /Script/Engine.KismetMaterialLibrary)
  (Rendering|Material|SetVectorParameterValue "/Game/Art/Materials/BaseMaterials/PC_BoxDissolver_Data.PC_BoxDissolver_Data" "Up" (Math|Conversions|ToLinearColor(Vector) (Math|Vector|GetUpVector _dissolver__shape_2)) :!class /Script/Engine.KismetMaterialLibrary))

(fn ConstructionScript
  (bind _dissolver__shape (Variables|Default|GetDissolver%20%20Shape))
  (bind _dissolver__shape_2 (Variables|Default|GetDissolver%20%20Shape))
  (Rendering|Material|SetVectorParameterValue "/Game/Art/Materials/BaseMaterials/PC_BoxDissolver_Data.PC_BoxDissolver_Data" "Location" (Math|Conversions|ToLinearColor(Vector) (Transformation|GetWorldLocation _dissolver__shape)) :!class /Script/Engine.KismetMaterialLibrary)
  (Rendering|Material|SetVectorParameterValue "/Game/Art/Materials/BaseMaterials/PC_BoxDissolver_Data.PC_BoxDissolver_Data" "Bounds" (Math|Conversions|ToLinearColor(Vector) (Transformation|GetWorldScale _dissolver__shape)) :!class /Script/Engine.KismetMaterialLibrary)
  (Rendering|Material|SetVectorParameterValue "/Game/Art/Materials/BaseMaterials/PC_BoxDissolver_Data.PC_BoxDissolver_Data" "Forward" (Math|Conversions|ToLinearColor(Vector) (Math|Vector|GetForwardVector _dissolver__shape_2)) :!class /Script/Engine.KismetMaterialLibrary)
  (Rendering|Material|SetVectorParameterValue "/Game/Art/Materials/BaseMaterials/PC_BoxDissolver_Data.PC_BoxDissolver_Data" "Right" (Math|Conversions|ToLinearColor(Vector) (Math|Vector|GetRightVector _dissolver__shape_2)) :!class /Script/Engine.KismetMaterialLibrary)
  (Rendering|Material|SetVectorParameterValue "/Game/Art/Materials/BaseMaterials/PC_BoxDissolver_Data.PC_BoxDissolver_Data" "Up" (Math|Conversions|ToLinearColor(Vector) (Math|Vector|GetUpVector _dissolver__shape_2)) :!class /Script/Engine.KismetMaterialLibrary))