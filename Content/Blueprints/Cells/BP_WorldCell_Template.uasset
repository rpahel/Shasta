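; BP_WorldCell_Template is a world cell template that drives a box dissolve effect from its DissolverShape component.
; UpdateDissolveMaterial writes the shape's world location and scale to the Location and Bounds vectors of the PC_BoxDissolver_Data material parameter collection.
; It runs from the construction script and on every Tick, so materials reading the collection follow the shape in editor and at runtime.
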(event EventTick
  (params (DeltaSeconds :type Float%20%28single-precision%29))
  (CallFunction|UpdateDissolveMaterial))

(fn ConstructionScript
  (CallFunction|UpdateDissolveMaterial))

(fn UpdateDissolveMaterial
  (bind _dissolvershape (Variables|Default|GetDissolverShape))
  (Utilities|IsValid _dissolvershape
    (:Is%20Valid
      (Rendering|Material|SetVectorParameterValue "/Game/Art/Materials/BaseMaterials/PC_BoxDissolver_Data.PC_BoxDissolver_Data" "Location" (Math|Conversions|ToLinearColor(Vector) (Transformation|GetWorldLocation _dissolvershape)) :!class /Script/Engine.KismetMaterialLibrary)
      (Rendering|Material|SetVectorParameterValue "/Game/Art/Materials/BaseMaterials/PC_BoxDissolver_Data.PC_BoxDissolver_Data" "Bounds" (Math|Conversions|ToLinearColor(Vector) (Transformation|GetWorldScale _dissolvershape)) :!class /Script/Engine.KismetMaterialLibrary))))